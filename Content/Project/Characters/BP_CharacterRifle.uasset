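; Rifle-armed character Blueprint that fires projectiles from its weapon.
; The construction script attaches the Weapon component to the mesh's hand_r socket, keeping relative transforms.
; Its Firing function extends the parent's logic by spawning a heavily scaled-down BP_Projectile at the location and rotation of the ArrowWeapon component.
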(fn `Firing`
  (bind _arrowweapon (`self.ArrowWeapon`))
  (`parent.Firing`)
  (`|SpawnActorFromClass` "/Game/Project/Weapons/BP_Projectile.BP_Projectile_C" (`KismetMathLibrary.MakeTransform` (`SceneComponent.K2_GetComponentLocation` _arrowweapon) (`SceneComponent.K2_GetComponentRotation` _arrowweapon) (* (1.0 1.0 1.0) 0.03)) "Undefined" "OverrideRootScale" null null))

(fn `UserConstructionScript`
  (`SceneComponent.K2_AttachToComponent` (`self.Weapon`) (`self.Mesh`) "hand_r" "KeepRelative" "KeepRelative" "KeepRelative" true))