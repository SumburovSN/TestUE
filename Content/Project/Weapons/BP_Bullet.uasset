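; BP_Bullet is a physics-driven projectile that damages pawns it hits.
; On BeginPlay it launches its sphere collision along its forward vector at a fixed speed.
; On hit it applies damage to a Pawn or otherwise spawns a steam particle effect without auto-destroy, then destroys itself.
; An alternative BP_DecalBullet impact spawn is left unconnected and never runs.
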(event `self.ReceiveBeginPlay`
  (bind _spherecollision (`self.SphereCollision`))
  ;[1 1 1] Bullet has been shooted
  (`PrimitiveComponent.SetPhysicsLinearVelocity` _spherecollision (* (`SceneComponent.GetForwardVector` _spherecollision) 3000.0) false "None"))

(event `self.SphereCollision.OnComponentHit`
  (params (HitComponent :type "PrimitiveComponent Object Reference") (OtherActor :type "Actor Object Reference") (OtherComp :type "PrimitiveComponent Object Reference") (NormalImpulse :type "Vector Structure") (Hit :type "HitResult Structure (by ref)"))
  ;[1 1 1] Comment
  (bind _aspawn (cast `Pawn` OtherActor)
    (:`then`
      (`GameplayStatics.ApplyDamage` _aspawn 25.0))
    (:`CastFailed`
      (`GameplayStatics.SpawnEmitterAtLocation` "/Game/Project/Effects/P_Steam_Lit.P_Steam_Lit" (`SceneComponent.K2_GetComponentLocation` HitComponent) (struct) (1.0 1.0 1.0) false)))
  (`self.K2_DestroyActor`))

(fn `UserConstructionScript`)